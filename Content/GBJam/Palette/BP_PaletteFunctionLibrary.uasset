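; Blueprint function library that exposes the active game palette's Background, Foreground, Highlight and Object colors.
; Each getter reads its vector parameter from the MPC_ActivePalette material parameter collection and returns it as either a Linear Color or a Slate Color.
; Values round-trip through an 8-bit Color without sRGB encoding, then back to Linear Color, so the stored values are treated as sRGB.
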(fn GetBackgroundColorSlate
  (bind _returnvalue (Rendering|Material|GetVectorParameterValue 0 "/Game/GBJam/Palette/MPC_ActivePalette.MPC_ActivePalette" "Background" :!class /Script/Engine.KismetMaterialLibrary))
  (return (Utilities|Struct|MakeSlateColor (Math|Conversions|ToLinearColor(Color) (Math|Conversions|ToColor(LinearColor) _returnvalue false)))))

(fn GetForegroundColorSlate
  (bind _returnvalue (Rendering|Material|GetVectorParameterValue 0 "/Game/GBJam/Palette/MPC_ActivePalette.MPC_ActivePalette" "Foreground" :!class /Script/Engine.KismetMaterialLibrary))
  (return (Utilities|Struct|MakeSlateColor (Math|Conversions|ToLinearColor(Color) (Math|Conversions|ToColor(LinearColor) _returnvalue false)))))

(fn GetForegroundColorLinear
  (bind _returnvalue (Rendering|Material|GetVectorParameterValue 0 "/Game/GBJam/Palette/MPC_ActivePalette.MPC_ActivePalette" "Foreground" :!class /Script/Engine.KismetMaterialLibrary))
  (return (Math|Conversions|ToLinearColor(Color) (Math|Conversions|ToColor(LinearColor) _returnvalue false))))

(fn GetBackgroundColorLinear
  (bind _returnvalue (Rendering|Material|GetVectorParameterValue 0 "/Game/GBJam/Palette/MPC_ActivePalette.MPC_ActivePalette" "Background" :!class /Script/Engine.KismetMaterialLibrary))
  (return (Math|Conversions|ToLinearColor(Color) (Math|Conversions|ToColor(LinearColor) _returnvalue false))))

(fn GetHighlightColorLinear
  (bind _returnvalue (Rendering|Material|GetVectorParameterValue 0 "/Game/GBJam/Palette/MPC_ActivePalette.MPC_ActivePalette" "Highlight" :!class /Script/Engine.KismetMaterialLibrary))
  (return (Math|Conversions|ToLinearColor(Color) (Math|Conversions|ToColor(LinearColor) _returnvalue false))))

(fn GetHighlightColorSlate
  (bind _returnvalue (Rendering|Material|GetVectorParameterValue 0 "/Game/GBJam/Palette/MPC_ActivePalette.MPC_ActivePalette" "Highlight" :!class /Script/Engine.KismetMaterialLibrary))
  (return (Utilities|Struct|MakeSlateColor (Math|Conversions|ToLinearColor(Color) (Math|Conversions|ToColor(LinearColor) _returnvalue false)))))

(fn GetObjectColorLinear
  (bind _returnvalue (Rendering|Material|GetVectorParameterValue 0 "/Game/GBJam/Palette/MPC_ActivePalette.MPC_ActivePalette" "Object" :!class /Script/Engine.KismetMaterialLibrary))
  (return (Math|Conversions|ToLinearColor(Color) (Math|Conversions|ToColor(LinearColor) _returnvalue false))))

(fn GetObjectColorSlate
  (bind _returnvalue (Rendering|Material|GetVectorParameterValue 0 "/Game/GBJam/Palette/MPC_ActivePalette.MPC_ActivePalette" "Object" :!class /Script/Engine.KismetMaterialLibrary))
  (return (Utilities|Struct|MakeSlateColor (Math|Conversions|ToLinearColor(Color) (Math|Conversions|ToColor(LinearColor) _returnvalue false)))))