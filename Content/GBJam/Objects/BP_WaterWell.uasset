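; BP_WaterWell is an examinable world object that shows flavor text about a water source.
; Its InteractRadius overlap events register and unregister it as an interactable when the player character enters or leaves.
; Interact shows one of two message pairs based on the Poisoned flag: poisoned water, or a water pipe someone may survive on.
; It supplies an examine prompt and always reports itself unlocked.
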(event OnComponentBeginOverlap(InteractRadius)
  (params (OverlappedComponent :type Primitive%20Component%20Object%20Reference) (OtherActor :type Actor%20Object%20Reference) (OtherComp :type Primitive%20Component%20Object%20Reference) (OtherBodyIndex :type Integer) (bFromSweep :type Boolean) (SweepResult :type Hit%20Result%20Structure%20%28by%20ref%29))
  (Utilities|Casting|CastToBP_PlayerCharacter OtherActor)
  (Class|GBGameplayStatics|AddInteractable self))

(event OnComponentEndOverlap(InteractRadius)
  (params (OverlappedComponent :type Primitive%20Component%20Object%20Reference) (OtherActor :type Actor%20Object%20Reference) (OtherComp :type Primitive%20Component%20Object%20Reference) (OtherBodyIndex :type Integer))
  (Utilities|Casting|CastToBP_PlayerCharacter OtherActor)
  (Class|GBGameplayStatics|RemoveInteractable self))

(event EventBeginPlay)

(event Collision|EventActorBeginOverlap
  (params (OtherActor :type Actor%20Object%20Reference)))

(event EventTick
  (params (DeltaSeconds :type Float%20%28single-precision%29)))

(event EventInteract
  (if (Variables|Default|GetPoisoned)
    (Class|GBGameplayStatics|ShowMessageBox "The water is poisoned.")
    (Class|GBGameplayStatics|ShowMessageBox "Everything is dead.")
    (else
      (Class|GBGameplayStatics|ShowMessageBox "Its a water pipe.")
      (Class|GBGameplayStatics|ShowMessageBox "Maybe they survive on this?"))))

(fn ConstructionScript)

(fn GetPrompt
  (return "Z - Examine"))

(fn IsLocked
  (return false))