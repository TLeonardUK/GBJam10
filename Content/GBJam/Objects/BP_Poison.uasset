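; BP_Poison is a pickup quest item that poisons the water well to kill the plants.
; Box overlap registers it as an interactable; interacting disables the box and adds it to the player's inventory.
; It overrides the well's interaction prompt.
; Use, within PoisonRadius of the well, sets its Poisoned flag, destroys all actors of three enemy classes and directs the player to the owner to finish the job.
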(event OnComponentBeginOverlap(Box)
  (params (OverlappedComponent :type Primitive%20Component%20Object%20Reference) (OtherActor :type Actor%20Object%20Reference) (OtherComp :type Primitive%20Component%20Object%20Reference) (OtherBodyIndex :type Integer) (bFromSweep :type Boolean) (SweepResult :type Hit%20Result%20Structure%20%28by%20ref%29))
  (Utilities|Casting|CastToBP_PlayerCharacter OtherActor)
  (Class|GBGameplayStatics|AddInteractable self))

(event OnComponentEndOverlap(Box)
  (params (OverlappedComponent :type Primitive%20Component%20Object%20Reference) (OtherActor :type Actor%20Object%20Reference) (OtherComp :type Primitive%20Component%20Object%20Reference) (OtherBodyIndex :type Integer))
  (Utilities|Casting|CastToBP_PlayerCharacter OtherActor)
  (Class|GBGameplayStatics|RemoveInteractable self))

(event EventBeginPlay)

(event Collision|EventActorBeginOverlap
  (params (OtherActor :type Actor%20Object%20Reference)))

(event EventTick
  (params (DeltaSeconds :type Float%20%28single-precision%29)))

(event EventInteract
  (Class|GBGameplayStatics|ShowMessageBox "You picked up a box of poison.")
  ;[1 1 1] Disable interaction box
  (Collision|SetCollisionEnabled (Variables|Default|GetBox) "NoCollision")
  (Class|GBGameplayStatics|RemoveInteractable self)
  ;[1 1 1] Attach to player
  (bind _asbp_player_character (Utilities|Casting|CastToBP_PlayerCharacter (Game|GetPlayerCharacter 0)))
  (Class|GBJamCharacter|AddItem _asbp_player_character self 1)
  (Audio|PlaySound2D "/Game/GBJam/SFX/pickupItem.pickupItem" 1.0 1.0 0.0 0 0))

(event EventEquip
  (Rendering|Material|SetMaterial (Variables|Default|GetStaticMesh) 0 "/Game/GBJam/Materials/MATI_Luminance10Emissive.MATI_Luminance10Emissive"))

(event EventUnequip)

(fn ConstructionScript)

(fn GetAttachmentOffset
  (return "25.000000,0.000000,0.000000"))

(fn GetDescription
  (return "Water soluble poison thats deadly to plants."))

(fn GetIcon
  (return "/Game/GBJam/Textures/Icons/MATI_Poison.MATI_Poison"))

(fn GetName
  (return "Poison"))

(fn GetOverrideInteractablePrompt
  (params (Other :type Actor%20Object%20Reference))
  (return "Z - Poison The Well"))

(fn GetPrompt
  (return "Z - Pickup"))

(fn ShouldOverrideInteractable
  (params (Other :type Actor%20Object%20Reference))
  (Utilities|Casting|CastToBP_WaterWell Other
    (:then
      (return true))
    (:CastFailed
      (return false))))

(fn Use
  (bind _returnvalue (Actor|GetActorOfClass "/Game/GBJam/Objects/BP_WaterWell.BP_WaterWell_C"))
  (if (<= (Transformation|GetDistanceTo _returnvalue self) (Variables|Default|GetPoisonRadius))
    (Audio|PlaySound2D "/Game/GBJam/SFX/explosion.explosion" 1.0 1.0 0.0 0 0)
    (Variables|/Game/GBJam/Objects/BP_WaterWell.BP_WaterWell_C|SetPoisoned _returnvalue true)
    (Class|GBGameplayStatics|ShowMessageBox "You poisoned the water.")
    (Class|GBGameplayStatics|ShowMessageBox "You hear the sound of plants dieing.")
    (Class|GBGameplayStatics|ShowMessageBox "...")
    (Class|GBGameplayStatics|ShowMessageBox "Talk to the owner to complete the job.")
    (bind _outactors (Actor|GetAllActorsOfClass "/Game/GBJam/Objects/Enemies/BP_Enemy.BP_Enemy_C"))
    (for _array_element _outactors
      (Actor|DestroyActor _array_element))
    (bind _outactors_2 (Actor|GetAllActorsOfClass "/Game/GBJam/Objects/Enemies/AOE/BP_Enemy_AOE.BP_Enemy_AOE_C"))
    (for _array_element_2 _outactors_2
      (Actor|DestroyActor _array_element_2))
    (bind _outactors_3 (Actor|GetAllActorsOfClass "/Game/GBJam/Objects/Enemies/Shooter/BP_Enemy_Shooter.BP_Enemy_Shooter_C"))
    (for _array_element_3 _outactors_3
      (Actor|DestroyActor _array_element_3))
    (return true)
    (else
      (Class|GBGameplayStatics|ShowMessageBox "Nothing to poison.")
      (return false))))