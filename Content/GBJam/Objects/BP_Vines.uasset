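; BP_Vines is a vine obstacle that the player can examine for a hint that extreme light may make it shrink.
; Overlap with its InteractBox registers or removes it as an interactable for BP_PlayerCharacter, with an examine prompt and message boxes on interaction.
; When flashbombed, it destroys itself if the source is within both a vertical and an overall distance threshold.
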(event OnComponentBeginOverlap(InteractBox)
  (params (OverlappedComponent :type Primitive%20Component%20Object%20Reference) (OtherActor :type Actor%20Object%20Reference) (OtherComp :type Primitive%20Component%20Object%20Reference) (OtherBodyIndex :type Integer) (bFromSweep :type Boolean) (SweepResult :type Hit%20Result%20Structure%20%28by%20ref%29))
  (Utilities|Casting|CastToBP_PlayerCharacter OtherActor)
  (Class|GBGameplayStatics|AddInteractable self))

(event OnComponentEndOverlap(InteractBox)
  (params (OverlappedComponent :type Primitive%20Component%20Object%20Reference) (OtherActor :type Actor%20Object%20Reference) (OtherComp :type Primitive%20Component%20Object%20Reference) (OtherBodyIndex :type Integer))
  (Utilities|Casting|CastToBP_PlayerCharacter OtherActor)
  (Class|GBGameplayStatics|RemoveInteractable self))

(event EventBeginPlay)

(event Collision|EventActorBeginOverlap
  (params (OtherActor :type Actor%20Object%20Reference)))

(event EventTick
  (params (DeltaSeconds :type Float%20%28single-precision%29)))

(event EventFlashbombed
  (params (Source :type Actor%20Object%20Reference))
  (bind _self self)
  (if (and (< (Math|Float|Absolute(Float) (- (.Z (Class|KismetMathLibrary|BreakVector3f (Transformation|GetActorLocation Source))) (.Z (Class|KismetMathLibrary|BreakVector3f (Transformation|GetActorLocation _self))))) (Variables|Default|GetFlashbombDestroyZDistance)) (< (Transformation|GetDistanceTo Source _self) (Variables|Default|GetFlashbombDestroyDistance)))
    (Actor|DestroyActor)))

(event EventInteract
  (Class|GBGameplayStatics|ShowMessageBox "Looks like some kind of vines.")
  (Class|GBGameplayStatics|ShowMessageBox "Extreme light may make them shrink."))

(fn ConstructionScript)

(fn GetPrompt
  (return "Z - Examine"))