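; BP_Flashbomb is a pickup item that gives the player a count of throwable flashbombs.
; A box overlap registers it as an interactable; interacting optionally shows messages, disables the box and adds the item to the player.
; Equipping applies an emissive material to its mesh.
; Using it spawns a BP_FlashbombProjectile just ahead of the item, launches it forward with a velocity-change impulse and plays a throw sound.
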(event OnComponentBeginOverlap(Box)
  (params (OverlappedComponent :type Primitive%20Component%20Object%20Reference) (OtherActor :type Actor%20Object%20Reference) (OtherComp :type Primitive%20Component%20Object%20Reference) (OtherBodyIndex :type Integer) (bFromSweep :type Boolean) (SweepResult :type Hit%20Result%20Structure%20%28by%20ref%29))
  (Utilities|Casting|CastToBP_PlayerCharacter OtherActor)
  (Class|GBGameplayStatics|AddInteractable self))

(event OnComponentEndOverlap(Box)
  (params (OverlappedComponent :type Primitive%20Component%20Object%20Reference) (OtherActor :type Actor%20Object%20Reference) (OtherComp :type Primitive%20Component%20Object%20Reference) (OtherBodyIndex :type Integer))
  (Utilities|Casting|CastToBP_PlayerCharacter OtherActor)
  (Class|GBGameplayStatics|RemoveInteractable self))

(event Custom|Use_1_1)

(event EventBeginPlay)

(event Collision|EventActorBeginOverlap
  (params (OtherActor :type Actor%20Object%20Reference)))

(event EventTick
  (params (DeltaSeconds :type Float%20%28single-precision%29)))

(event EventInteract
  (if (Variables|Default|GetShowMesage)
    (Class|GBGameplayStatics|ShowMessageBox "You picked up flashbombs. 
Press Z to throw")
    (Class|GBGameplayStatics|ShowMessageBox "They produce exteme light and sound."))
  ;[1 1 1] Disable interaction box
  (Collision|SetCollisionEnabled (Variables|Default|GetBox) "NoCollision")
  (Class|GBGameplayStatics|RemoveInteractable self)
  ;[1 1 1] Attach to player
  (bind _asbp_player_character (Utilities|Casting|CastToBP_PlayerCharacter (Game|GetPlayerCharacter 0)))
  (Class|GBJamCharacter|AddItem _asbp_player_character self (Variables|Default|GetFlashbombCount))
  (Audio|PlaySound2D "/Game/GBJam/SFX/pickupItem.pickupItem" 1.0 1.0 0.0 0 0))

(event EventEquip
  (Rendering|Material|SetMaterial (Variables|Default|GetStaticMesh) 0 "/Game/GBJam/Materials/MATI_Luminance10Emissive.MATI_Luminance10Emissive"))

(event EventUnequip)

(fn ConstructionScript)

(fn GetAttachmentOffset
  (return "25.000000,0.000000,0.000000"))

(fn GetDescription
  (return "Produces a bright flash after a short delay."))

(fn GetIcon
  (return "/Game/GBJam/Textures/Icons/MATI_FlashbombIcon.MATI_FlashbombIcon"))

(fn GetName
  (return "Flashbomb"))

(fn GetOverrideInteractablePrompt
  (params (Other :type Actor%20Object%20Reference))
  (return ""))

(fn GetPrompt
  (return "Z - Pickup"))

(fn ShouldOverrideInteractable
  (params (Other :type Actor%20Object%20Reference))
  (return false))

(fn Use
  (bind _returnvalue (Game|SpawnActorfromClass "/Game/GBJam/Objects/BP_FlashbombProjectile.BP_FlashbombProjectile_C" (Math|Transform|ComposeTransforms (Math|Transform|MakeTransform "45.000000,0.000000,0.000000") (Transformation|GetActorTransform)) "Undefined" 0 0))
  (Physics|AddImpulse (Variables|/Game/GBJam/Objects/BP_FlashbombProjectile.BP_FlashbombProjectile_C|GetStaticMesh _returnvalue) (* (Math|Vector|GetForwardVector (Variables|/Game/GBJam/Objects/BP_FlashbombProjectile.BP_FlashbombProjectile_C|GetStaticMesh _returnvalue)) "500.000000,500.000000,500.000000") "None" true)
  (Audio|PlaySound2D "/Game/GBJam/SFX/throw.throw" 1.0 1.0 0.0 0 0)
  (return true))