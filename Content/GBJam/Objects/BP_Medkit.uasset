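; Medkit pickup item that the player collects and later uses to heal one heart.
; Overlapping its box registers it as an interactable; interacting shows a message, disables the box and adds it to the player's inventory with a pickup sound.
; Use heals through the player's GBHealthComponent and reports success, or shows a message and fails at full health.
; It also supplies name, icon, description, prompt and attachment offset, and swaps its mesh material when equipped.
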(event OnComponentBeginOverlap(Box)
  (params (OverlappedComponent :type Primitive%20Component%20Object%20Reference) (OtherActor :type Actor%20Object%20Reference) (OtherComp :type Primitive%20Component%20Object%20Reference) (OtherBodyIndex :type Integer) (bFromSweep :type Boolean) (SweepResult :type Hit%20Result%20Structure%20%28by%20ref%29))
  (Utilities|Casting|CastToBP_PlayerCharacter OtherActor)
  (Class|GBGameplayStatics|AddInteractable self))

(event OnComponentEndOverlap(Box)
  (params (OverlappedComponent :type Primitive%20Component%20Object%20Reference) (OtherActor :type Actor%20Object%20Reference) (OtherComp :type Primitive%20Component%20Object%20Reference) (OtherBodyIndex :type Integer))
  (Utilities|Casting|CastToBP_PlayerCharacter OtherActor)
  (Class|GBGameplayStatics|RemoveInteractable self))

(event EventBeginPlay)

(event Collision|EventActorBeginOverlap
  (params (OtherActor :type Actor%20Object%20Reference)))

(event EventTick
  (params (DeltaSeconds :type Float%20%28single-precision%29)))

(event EventInteract
  (Class|GBGameplayStatics|ShowMessageBox "You picked up a medkit 
Heals one heart.")
  ;[1 1 1] Disable interaction box
  (Collision|SetCollisionEnabled (Variables|Default|GetBox) "NoCollision")
  (Class|GBGameplayStatics|RemoveInteractable self)
  ;[1 1 1] Attach to player
  (bind _asbp_player_character (Utilities|Casting|CastToBP_PlayerCharacter (Game|GetPlayerCharacter 0)))
  (Class|GBJamCharacter|AddItem _asbp_player_character self 1)
  (Audio|PlaySound2D "/Game/GBJam/SFX/pickupItem.pickupItem" 1.0 1.0 0.0 0 0))

(event EventEquip
  (Rendering|Material|SetMaterial (Variables|Default|GetStaticMesh) 0 "/Game/GBJam/Materials/MATI_Luminance10Emissive.MATI_Luminance10Emissive"))

(event EventUnequip)

(fn ConstructionScript)

(fn GetAttachmentOffset
  (return "25.000000,0.000000,0.000000"))

(fn GetDescription
  (return "Can be used to heal a single heart of damage."))

(fn GetIcon
  (return "/Game/GBJam/Textures/Icons/MATI_Medkit.MATI_Medkit"))

(fn GetName
  (return "Medkit"))

(fn GetOverrideInteractablePrompt
  (params (Other :type Actor%20Object%20Reference))
  (return ""))

(fn GetPrompt
  (return "Z - Pickup"))

(fn ShouldOverrideInteractable
  (params (Other :type Actor%20Object%20Reference))
  (return false))

(fn Use
  (bind _returnvalue (Game|GetPlayerCharacter 0))
  (bind _returnvalue_2 (Actor|GetComponentbyClass _returnvalue "/Script/GBJam.GBHealthComponent"))
  (if (< (Variables|/Script/GBJam.GBHealthComponent|GetHealth _returnvalue_2) (Variables|/Script/GBJam.GBHealthComponent|GetMaxHealth _returnvalue_2))
    (Class|GBHealthComponent|Heal _returnvalue_2 1.0)
    (return true)
    (else
      (Class|GBGameplayStatics|ShowMessageBox "You are at full health.")
      (return false))))