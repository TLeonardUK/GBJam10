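; Flashbomb projectile that explodes on a three-second timer, stunning the view with a palette flash and alerting nearby actors.
; On explosion it plays a sound and calls Flashbombed on every BPI_NotifiedOfFlashbomb actor within EffectRadius.
; A camera dot-product check, with no occlusion trace, decides whether the player sees the flash.
; If so, GBPaletteSubSystem swaps to the Explode palette, then starts a stepped transition to Default before the actor destroys itself.
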(event Custom|Explode
  (bind _returnvalue (Subsystems|GetGBPaletteSubSystem))
  (Audio|PlaySoundatLocation "/Game/GBJam/SFX/explosion.explosion" (Transformation|GetWorldLocation (Variables|Default|GetStaticMesh)) "0, 0, 0" 1.0 1.0 0.0 0 0 0 0)
  (CallFunction|NotifyEnemies)
  (if (CallFunction|PlayerCanSeeFlash)
    (bind _returnvalue_2 (Utilities|GetDataTableRow "/Game/GBJam/Palette/DT_Palettes.DT_Palettes" "Explode")
      (:then
        (Class|GBPaletteSubSystem|SetPalette _returnvalue _returnvalue_2)
        (Utilities|FlowControl|Delay 0.5)
        (bind _returnvalue_3 (Utilities|GetDataTableRow "/Game/GBJam/Palette/DT_Palettes.DT_Palettes" "Default")
          (:then
            (Class|GBPaletteSubSystem|TransitionPalette _returnvalue _returnvalue_3 5 0.5)
            (Utilities|FlowControl|Delay 0.5))))))
  (Actor|DestroyActor))

(event Custom|NotifyEnemies
  (bind _outactors (Actor|GetAllActorsOfClass "/Script/Engine.Actor"))
  (for _array_element _outactors
    (bind _asbpi_notified_of_flashbomb (Utilities|Casting|CastToBPI_NotifiedOfFlashbomb _array_element))
    (if (< (Transformation|GetDistanceTo _array_element) (Variables|Default|GetEffectRadius))
      (Default|Flashbombed _asbpi_notified_of_flashbomb self))))

(event EventBeginPlay
  (Utilities|Time|SetTimerbyEvent (delegate Custom|Explode) 3.0))

(event Collision|EventActorBeginOverlap
  (params (OtherActor :type Actor%20Object%20Reference)))

(event EventTick
  (params (DeltaSeconds :type Float%20%28single-precision%29)))

(fn ConstructionScript)

(fn PlayerCanSeeFlash
  (bind _returnvalue (Game|GetPlayerCameraManager 0))
  (return (> (Math|Vector|DotProduct (Math|Vector|GetForwardVector (Camera|GetCameraRotation _returnvalue)) (Math|Vector|Normalize (- (Transformation|GetWorldLocation (Variables|Default|GetStaticMesh)) (Camera|GetCameraLocation _returnvalue)))) 0.4)))