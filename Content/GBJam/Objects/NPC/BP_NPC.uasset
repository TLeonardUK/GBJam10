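; BP_NPC is the quest-giver NPC who asks the player for help, hands over a key and ends the game once the BP_WaterWell is poisoned.
; An arm-waving timeline loops from BeginPlay until the intro dialogue drops the arm and triggers the key pickup message.
; An overlap box registers it as an interactable, and later talks step through follow-up lines, holding on the last.
; Message-box sequencing uses zero-delay polling loops.
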(event OnComponentBeginOverlap(InteractBox)
  (params (OverlappedComponent :type Primitive%20Component%20Object%20Reference) (OtherActor :type Actor%20Object%20Reference) (OtherComp :type Primitive%20Component%20Object%20Reference) (OtherBodyIndex :type Integer) (bFromSweep :type Boolean) (SweepResult :type Hit%20Result%20Structure%20%28by%20ref%29))
  (Utilities|Casting|CastToBP_PlayerCharacter OtherActor)
  (Class|GBGameplayStatics|AddInteractable self))

(event OnComponentEndOverlap(InteractBox)
  (params (OverlappedComponent :type Primitive%20Component%20Object%20Reference) (OtherActor :type Actor%20Object%20Reference) (OtherComp :type Primitive%20Component%20Object%20Reference) (OtherBodyIndex :type Integer))
  (Utilities|Casting|CastToBP_PlayerCharacter OtherActor)
  (Class|GBGameplayStatics|RemoveInteractable self))

(event Custom|DropArm
  (bind _np_npc_arm (Variables|Default|GetNP_NPC_ARM))
  (Variables|Default|SetWaving false)
  (Utilities|FlowControl|Sequence
    (:then_0
      (bind _arm (Timeline|Wave%20Loop Stop)
        (:Update
          (Transformation|SetRelativeRotation _np_npc_arm (Math|Rotator|MakeRotator (.X (Class|KismetMathLibrary|BreakVector3f _arm)) (.Y (Class|KismetMathLibrary|BreakVector3f _arm)) (.Z (Class|KismetMathLibrary|BreakVector3f _arm))) false false))
        (:Finished
          (CallFunction|Wave))))
    (:then_1
      (bind _arm_2 (Timeline|Drop Play)
        (:Update
          (Transformation|SetRelativeRotation _np_npc_arm (Math|Rotator|MakeRotator (.X (Class|KismetMathLibrary|BreakVector3f _arm_2)) (.Y (Class|KismetMathLibrary|BreakVector3f _arm_2)) (.Z (Class|KismetMathLibrary|BreakVector3f _arm_2))) false false))))))

(event Custom|Wave
  (if (Variables|Default|GetWaving)
    (bind _arm (Timeline|Wave%20Loop PlayFromStart)
      (:Update
        (Transformation|SetRelativeRotation (Variables|Default|GetNP_NPC_ARM) (Math|Rotator|MakeRotator (.X (Class|KismetMathLibrary|BreakVector3f _arm)) (.Y (Class|KismetMathLibrary|BreakVector3f _arm)) (.Z (Class|KismetMathLibrary|BreakVector3f _arm))) false false))
      (:Finished
        (CallFunction|Wave)))))

(event EventBeginPlay
  (Variables|Default|SetWaving true)
  (CallFunction|Wave))

(event Collision|EventActorBeginOverlap
  (params (OtherActor :type Actor%20Object%20Reference)))

(event EventTick
  (params (DeltaSeconds :type Float%20%28single-precision%29)))

(event EventInteract
  (bind _returnvalue (Actor|GetActorOfClass "/Game/GBJam/Objects/BP_WaterWell.BP_WaterWell_C"))
  (if (Variables|/Game/GBJam/Objects/BP_WaterWell.BP_WaterWell_C|GetPoisoned _returnvalue)
    (Class|GBGameplayStatics|ShowMessageBox "All .. Dead.")
    (Class|GBGameplayStatics|ShowMessageBox "...")
    (Class|GBGameplayStatics|ShowMessageBox "...")
    (Class|GBGameplayStatics|ShowMessageBox "... thank you ...")
    (bind _returnvalue_2 (Class|GBGameplayStatics|IsMessageBoxOpen :!label _label))
    (if _returnvalue_2
      (Utilities|FlowControl|Delay 0.0)
      (goto _label)
      (else
        (bind _asbp_game_mode (Utilities|Casting|CastToBP_GameMode (Game|GetGameMode)))
        (Default|GameComplete _asbp_game_mode)))
    (elif (Variables|Default|GetPlayedIntro)
      (Class|GBGameplayStatics|ShowMessageBox (Utilities|Array|Get(acopy) (Variables|Default|GetAfterIntroMessages) (Variables|Default|GetAfterIntroMessageIndex)))
      (Variables|Default|SetAfterIntroMessageIndex (Math|Integer|Clamp(Integer) (+ (Variables|Default|GetAfterIntroMessageIndex) 1) 0 (- (Utilities|Array|Length (Variables|Default|GetAfterIntroMessages)) 1)))
      (else
        (Variables|Default|SetPlayedIntro true)
        (Class|GBGameplayStatics|ShowMessageBox "Hello.")
        (Class|GBGameplayStatics|ShowMessageBox "Please Help.")
        (Class|GBGameplayStatics|ShowMessageBox "My ... experiments ...")
        (Class|GBGameplayStatics|ShowMessageBox "Have gotten out of control ...")
        (Class|GBGameplayStatics|ShowMessageBox "I need you to help ...")
        (Class|GBGameplayStatics|ShowMessageBox "Please ...")
        (Class|GBGameplayStatics|ShowMessageBox "Take this key, it will get you inside.")
        (CallFunction|DropArm)
        (bind _returnvalue_3 (Class|GBGameplayStatics|IsMessageBoxOpen :!label _label_2))
        (if _returnvalue_3
          (Utilities|FlowControl|Delay 0.0)
          (goto _label_2)
          (else
            (Class|GBInteractable|Interact(Message) (Variables|Default|GetKeyPickup))
            (bind _returnvalue_4 (Class|GBGameplayStatics|IsMessageBoxOpen :!label _label_3))
            (if _returnvalue_4
              (Utilities|FlowControl|Delay 0.0)
              (goto _label_3)
              (else
                (Utilities|FlowControl|Delay 1.5)
                (Class|GBGameplayStatics|ShowMessageBox "Thank you ...")))))))))

(fn ConstructionScript)

(fn GetPrompt
  (return "Z - Speak"))