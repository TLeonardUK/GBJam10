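; BP_Door is an interactable hinged door that the player can open, close and find locked.
; Its InteractRadius overlaps add or remove it as an interactable for BP_PlayerCharacter, and GetPrompt reflects its open state.
; Interact shows a locked message or toggles a timeline that rotates DoorPivot, with ReverseOpening flipping the swing direction.
; OnUnlocked clears the lock with a message and sound, while IsLocked exposes that state.
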(event OnComponentBeginOverlap(InteractRadius)
  (params (OverlappedComponent :type Primitive%20Component%20Object%20Reference) (OtherActor :type Actor%20Object%20Reference) (OtherComp :type Primitive%20Component%20Object%20Reference) (OtherBodyIndex :type Integer) (bFromSweep :type Boolean) (SweepResult :type Hit%20Result%20Structure%20%28by%20ref%29))
  (Utilities|Casting|CastToBP_PlayerCharacter OtherActor)
  (Class|GBGameplayStatics|AddInteractable self))

(event OnComponentEndOverlap(InteractRadius)
  (params (OverlappedComponent :type Primitive%20Component%20Object%20Reference) (OtherActor :type Actor%20Object%20Reference) (OtherComp :type Primitive%20Component%20Object%20Reference) (OtherBodyIndex :type Integer))
  (Utilities|Casting|CastToBP_PlayerCharacter OtherActor)
  (Class|GBGameplayStatics|RemoveInteractable self))

(event EventBeginPlay)

(event Collision|EventActorBeginOverlap
  (params (OtherActor :type Actor%20Object%20Reference)))

(event EventTick
  (params (DeltaSeconds :type Float%20%28single-precision%29)))

(event EventInteract
  (if (Variables|Default|GetIsDoorLocked)
    (Class|GBGameplayStatics|ShowMessageBox "The door is locked. 
You need a key to open.")
    (else
      (Variables|Default|SetIsOpen (not (Variables|Default|GetIsOpen)))
      (Audio|PlaySound2D "/Game/GBJam/SFX/openDoor4.openDoor4" 1.0 1.0 0.0 0 0)
      (if (Variables|Default|GetIsOpen)
        (bind _doorrotation (Timeline|OpenTimeline Play)
          (:Update
            (Transformation|SetRelativeRotation (Variables|Default|GetDoorPivot) (Math|Rotator|MakeRotator 0.0 0.0 (Math|Float|SelectFloat (* _doorrotation -1.0) _doorrotation (Variables|Default|GetReverseOpening))) false false)))
        (else
          (Timeline|OpenTimeline Reverse))))))

(event EventOnUnlocked
  (Variables|Default|SetIsDoorLocked false)
  (Class|GBGameplayStatics|ShowMessageBox "The door unlocked.")
  (Audio|PlaySound2D "/Game/GBJam/SFX/unlockDoor.unlockDoor" 1.0 1.0 0.0 0 0))

(fn ConstructionScript)

(fn GetPrompt
  (return (Utilities|String|SelectString "Z - Close Door" "Z - Open Door" (Variables|Default|GetIsOpen))))

(fn IsLocked
  (return (Variables|Default|GetIsDoorLocked)))