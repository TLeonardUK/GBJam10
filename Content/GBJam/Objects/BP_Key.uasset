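; BP_Key is a pickup item that the player adds to inventory, equips and uses to unlock nearby locked objects.
; A box overlap registers it as an interactable, and interacting disables the box and adds it to the player's items.
; Use scans all actors for a locked BPI_Lockable within UnlockRadius and unlocks the first found.
; Getters supply name, icon and prompts, including an unlock prompt override for locked targets.
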(event OnComponentBeginOverlap(Box)
  (params (OverlappedComponent :type Primitive%20Component%20Object%20Reference) (OtherActor :type Actor%20Object%20Reference) (OtherComp :type Primitive%20Component%20Object%20Reference) (OtherBodyIndex :type Integer) (bFromSweep :type Boolean) (SweepResult :type Hit%20Result%20Structure%20%28by%20ref%29))
  (Utilities|Casting|CastToBP_PlayerCharacter OtherActor)
  (Class|GBGameplayStatics|AddInteractable self))

(event OnComponentEndOverlap(Box)
  (params (OverlappedComponent :type Primitive%20Component%20Object%20Reference) (OtherActor :type Actor%20Object%20Reference) (OtherComp :type Primitive%20Component%20Object%20Reference) (OtherBodyIndex :type Integer))
  (Utilities|Casting|CastToBP_PlayerCharacter OtherActor)
  (Class|GBGameplayStatics|RemoveInteractable self))

(event Custom|Use_1_1)

(event EventBeginPlay)

(event Collision|EventActorBeginOverlap
  (params (OtherActor :type Actor%20Object%20Reference)))

(event EventTick
  (params (DeltaSeconds :type Float%20%28single-precision%29)))

(event EventInteract
  (Class|GBGameplayStatics|ShowMessageBox "You picked up a key 
Equip and use on doors to unlock.")
  ;[1 1 1] Disable interaction box
  (Collision|SetCollisionEnabled (Variables|Default|GetBox) "NoCollision")
  (Class|GBGameplayStatics|RemoveInteractable self)
  ;[1 1 1] Attach to player
  (bind _asbp_player_character (Utilities|Casting|CastToBP_PlayerCharacter (Game|GetPlayerCharacter 0)))
  (Class|GBJamCharacter|AddItem _asbp_player_character self 1)
  (Audio|PlaySound2D "/Game/GBJam/SFX/pickupItem.pickupItem" 1.0 1.0 0.0 0 0))

(event EventEquip
  (Rendering|Material|SetMaterial (Variables|Default|GetStaticMesh) 0 "/Game/GBJam/Materials/MATI_Luminance10Emissive.MATI_Luminance10Emissive"))

(event EventUnequip)

(fn ConstructionScript)

(fn GetAttachmentOffset
  (return "25.000000,0.000000,0.000000"))

(fn GetDescription
  (return "Opens a locked object"))

(fn GetIcon
  (return "/Game/GBJam/Textures/Icons/MATI_KeyIcon.MATI_KeyIcon"))

(fn GetName
  (return "Key"))

(fn GetOverrideInteractablePrompt
  (params (Other :type Actor%20Object%20Reference))
  (return "Z - Unlock"))

(fn GetPrompt
  (return "Z - Pickup"))

(fn ShouldOverrideInteractable
  (params (Other :type Actor%20Object%20Reference))
  (bind _asbpi_lockable (Utilities|Casting|CastToBPI_Lockable Other)
    (:then
      (bind _locked (Default|IsLocked _asbpi_lockable))
      (return _locked))
    (:CastFailed
      (return false))))

(fn Use
  (Variables|Default|SetUnlockSuccess false)
  (bind _outactors (Actor|GetAllActorsOfClass "/Script/Engine.Actor"))
  (bind _array_element (Utilities|Array|ForEachLoopwithBreak _outactors :!label _label)
    (:LoopBody
      (bind _asbpi_lockable (Utilities|Casting|CastToBPI_Lockable _array_element))
      (bind _locked (Default|IsLocked _asbpi_lockable))
      (if (and _locked (< (Transformation|GetDistanceTo _array_element self) (Variables|Default|GetUnlockRadius)))
        (Default|OnUnlocked _asbpi_lockable)
        (Variables|Default|SetUnlockSuccess true)
        (goto _label Break)))
    (:Completed
      (if (Variables|Default|GetUnlockSuccess)
        (return true)
        (else
          (Class|GBGameplayStatics|ShowMessageBox "Nothing to unlock.")
          (return false))))))