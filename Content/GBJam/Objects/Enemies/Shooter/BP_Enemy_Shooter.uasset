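; BP_Enemy_Shooter is an enemy that fires projectiles at a regular interval unless it is in light or in a flashbomb.
; BeginPlay starts a looping Attack timer with a configurable interval and start offset.
; Each attack checks IsActive, plays a sound, then spawns a BP_ShooterProjectile at SpawnLocation and launches it forward with a velocity-change impulse.
; A timeline animates the AoeTree component's scale on each shot.
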(event Custom|Attack
  (bind _spawn_location (Variables|Default|Getspawn_location))
  (bind _active (CallFunction|IsActive))
  (if _active
    (Audio|PlaySoundatLocation "/Game/GBJam/SFX/pew.pew" (Transformation|GetActorLocation) "0, 0, 0" 1.0 1.0 0.0 0 0 0 0)
    (bind _returnvalue (Game|SpawnActorfromClass "/Game/GBJam/Objects/Enemies/Shooter/BP_ShooterProjectile.BP_ShooterProjectile_C" (Math|Transform|MakeTransform (Transformation|GetWorldLocation _spawn_location) (Transformation|GetWorldRotation _spawn_location)) "AlwaysSpawn" 0 0))
    (Physics|AddImpulse (Variables|/Game/GBJam/Objects/Enemies/Shooter/BP_ShooterProjectile.BP_ShooterProjectile_C|GetSphere _returnvalue) (* (Math|Vector|GetForwardVector _spawn_location) "1500.000000,1500.000000,1500.000000") "None" true)
    (bind _scale (Timeline|AttackTimeline PlayFromStart)
      (:Update
        (Transformation|SetRelativeScale3D (Variables|Default|Getaoe_tree) (* _scale "0.500000,0.500000,0.500000"))))))

(event EventBeginPlay
  (Utilities|Time|SetTimerbyEvent (delegate Custom|Attack) (Variables|Default|GetAttackInterval) true (Variables|Default|GetAttackOffset)))

(event Collision|EventActorBeginOverlap
  (params (OtherActor :type Actor%20Object%20Reference)))

(event EventTick
  (params (DeltaSeconds :type Float%20%28single-precision%29)))

(fn ConstructionScript)

(fn IsActive
  (return (and (not (Variables|Default|GetInLight)) (not (Variables|Default|GetInFlashbomb)))))