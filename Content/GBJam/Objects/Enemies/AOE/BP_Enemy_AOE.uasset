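; BP_Enemy_AOE is an area-of-effect enemy that hurts the player while not lit by the flashlight or flashbombed.
; A looping attack timer plays sound and VFX and scales the AoeTree through a timeline.
; A separate looping timer damages the player tracked by DamageBox overlaps.
; IsActive gates both timers' effects, while flashlight changes also toggle the tree's custom depth and flashbombs disable it temporarily.
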(event OnComponentBeginOverlap(DamageBox)
  (params (OverlappedComponent :type Primitive%20Component%20Object%20Reference) (OtherActor :type Actor%20Object%20Reference) (OtherComp :type Primitive%20Component%20Object%20Reference) (OtherBodyIndex :type Integer) (bFromSweep :type Boolean) (SweepResult :type Hit%20Result%20Structure%20%28by%20ref%29))
  (bind _asbp_player_character (Utilities|Casting|CastToBP_PlayerCharacter OtherActor))
  (Variables|Default|SetPlayer _asbp_player_character))

(event OnComponentEndOverlap(DamageBox)
  (params (OverlappedComponent :type Primitive%20Component%20Object%20Reference) (OtherActor :type Actor%20Object%20Reference) (OtherComp :type Primitive%20Component%20Object%20Reference) (OtherBodyIndex :type Integer))
  (Utilities|Casting|CastToBP_PlayerCharacter OtherActor)
  (Variables|Default|SetPlayer 0))

(event Custom|Attack
  (bind _active (CallFunction|IsActive))
  (if _active
    (Audio|PlaySoundatLocation "/Game/GBJam/SFX/aoe.aoe" (Transformation|GetActorLocation) "0, 0, 0" 1.0 1.0 0.0 0 0 0 0)
    (bind _returnvalue (Niagara|SpawnSystemAttached "/Game/GBJam/Objects/Enemies/AOE/BP_AOE_FX.BP_AOE_FX" (Variables|Default|Getvfx_spawn_location) "None" "0, 0, 0" "0, 0, 0" "KeepRelativeOffset" true))
    (Rendering|SetRenderCustomDepth _returnvalue true)
    (bind _scale (Timeline|AttackTimeline PlayFromStart)
      (:Update
        (Transformation|SetRelativeScale3D (Variables|Default|Getaoe_tree) _scale)))))

(event Custom|ApplyDamage
  (bind _player (Variables|Default|GetPlayer))
  (bind _active (CallFunction|IsActive))
  (if _active
    (Utilities|IsValid _player
      (:Is%20Valid
        (Game|Damage|ApplyDamage _player 1.0 0 self "/Script/GBJam.GBDamageType_Enemy")))))

(event Custom|UpdateCustomDepth
  (bind _active (CallFunction|IsActive))
  (Rendering|SetRenderCustomDepth (Variables|Default|Getaoe_tree) _active))

(event Custom|ResetFlashbomb
  (Variables|Default|SetInFlashbomb false))

(event EventBeginPlay
  (Utilities|Time|SetTimerbyEvent (delegate Custom|Attack) (Variables|Default|GetAttackInterval) true)
  (Utilities|Time|SetTimerbyEvent (delegate Custom|ApplyDamage) (Variables|Default|GetDamageInterval) true))

(event Collision|EventActorBeginOverlap
  (params (OtherActor :type Actor%20Object%20Reference)))

(event EventTick
  (params (DeltaSeconds :type Float%20%28single-precision%29)))

(event EventSetinFlashlight
  (params (InFlashlight :type Boolean))
  (Variables|Default|SetInLight InFlashlight)
  (CallFunction|UpdateCustomDepth))

(event EventFlashbombed
  (params (Source :type Actor%20Object%20Reference))
  (Variables|Default|SetInFlashbomb true)
  (Utilities|Time|SetTimerbyEvent (delegate Custom|ResetFlashbomb) (Variables|Default|GetFlashbombDuration)))

(fn ConstructionScript)

(fn IsActive
  (return (and (not (Variables|Default|GetInLight)) (not (Variables|Default|GetInFlashbomb)))))