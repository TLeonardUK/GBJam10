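; BP_Enemy is the enemy character for GBJam, storing its spawn location and exposing functions for walk speed and visual state.
; Flashbomb and flashlight events are forwarded to BP_EnemyController as notifications.
; Flashbombed and blink states toggle custom depth rendering on the Tree component, with flashbombing also switching its stencil value.
; Starting a blink plays the Attack sound at the enemy's position.
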(event Custom|SetIsFlashbombed
  (params (Flashbombed :type Boolean))
  (bind _returnvalue (not Flashbombed))
  (bind _tree (Variables|Default|Gettree))
  (Rendering|SetRenderCustomDepth _tree _returnvalue)
  (Rendering|SetCustomDepthStencilValue _tree (Math|Integer|SelectInt 2 0 _returnvalue)))

(event EventBeginPlay
  (Variables|Default|SetBaseLocation (Transformation|GetActorLocation)))

(event Collision|EventActorBeginOverlap
  (params (OtherActor :type Actor%20Object%20Reference)))

(event EventTick
  (params (DeltaSeconds :type Float%20%28single-precision%29)))

(event EventFlashbombed
  (params (Source :type Actor%20Object%20Reference))
  (bind _asbp_enemy_controller (Utilities|Casting|CastToBP_EnemyController (Pawn|GetController)))
  (Default|NotifyFlashBombed _asbp_enemy_controller))

(event EventSetinFlashlight
  (params (InFlashlight :type Boolean))
  (bind _asbp_enemy_controller (Utilities|Casting|CastToBP_EnemyController (Pawn|GetController)))
  (Default|SetIsLightnear _asbp_enemy_controller InFlashlight))

(fn ConstructionScript)

(fn UpdateWalkSpeed
  (params (NewSpeed :type Float%20%28double-precision%29))
  (Variables|/Script/Engine.CharacterMovementComponent|SetMaxWalkSpeed (Variables|Character|GetCharacterMovement) NewSpeed))

(fn SetBlink
  (params (Blink :type Boolean))
  (if (!= (Variables|Default|GetBlinking) Blink)
    (Rendering|SetRenderCustomDepth (Variables|Default|Gettree) (not Blink))
    (bind _output_get (Variables|Default|SetBlinking Blink))
    (if _output_get
      (Audio|PlaySoundatLocation "/Game/GBJam/SFX/attack.attack" (Transformation|GetActorLocation) "0, 0, 0" 1.0 1.0 0.0 0 0 0 0))))