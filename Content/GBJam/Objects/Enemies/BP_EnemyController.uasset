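; AI controller for BP_Enemy that runs its behavior tree and feeds its blackboard with player detection, chase-range and flashbomb state.
; A perceived player counts only within a sense distance that depends on nearby light and eases faster up than down, so brief torch flicks go unnoticed.
; Losing the target starts a grace timer before clearing line of sight.
; Timers also drive enemy blinking and end the flashbomb effect.
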(event OnTargetPerceptionUpdated(AIPerception)
  (params (Actor :type Actor%20Object%20Reference) (Stimulus :type AI%20Stimulus%20Structure))
  (if (and (Actor|ActorHasTag Actor "Player") (.bSuccessfullySensed (Utilities|Struct|BreakAIStimulus Stimulus)))
    (Variables|Default|SetActivePerception Actor)
    (else
      (Variables|Default|SetActivePerception 0))))

(event Custom|StartEnemyTimer
  (bind _returnvalue (AI|GetBlackboard 0))
  (AI|Components|Blackboard|SetValueasBool _returnvalue (Variables|Default|GetHasLineOfSight) false)
  (AI|Components|Blackboard|SetValueasObject _returnvalue (Variables|Default|GetEnemyActor) 0)
  (Variables|Default|SetWasValidTarget false)
  (Utilities|Time|InvalidateTimerHandle (Variables|Default|GetEnemyTimer)))

(event Custom|Blink
  (bind _asbp_enemy (Utilities|Casting|CastToBP_Enemy (Pawn|GetControlledPawn)))
  (if (Variables|Default|GetShouldBlink)
    (Variables|Default|SetBlinked (not (Variables|Default|GetBlinked)))
    (Default|SetBlink _asbp_enemy (Variables|Default|GetBlinked))
    (else
      (Default|SetBlink _asbp_enemy false))))

(event EventBeginPlay
  (Utilities|Time|SetTimerbyEvent (delegate Custom|Blink) (Variables|Default|GetBlinkInterval) true))

(event EventTick
  (params (DeltaSeconds :type Float%20%28single-precision%29))
  (bind _returnvalue (AI|GetBlackboard 0))
  (bind _activeperception (Variables|Default|GetActivePerception))
  (Utilities|FlowControl|Sequence
    (:then_0
      (bind _valid (CallFunction|IsValidTarget _activeperception))
      (if (and (!= (Variables|Default|GetActivePerception) 0) _valid)
        (Utilities|Time|ClearandInvalidateTimerbyHandle (Variables|Default|GetEnemyTimer))
        (AI|Components|Blackboard|SetValueasBool _returnvalue (Variables|Default|GetHasLineOfSight) true)
        (AI|Components|Blackboard|SetValueasObject _returnvalue (Variables|Default|GetEnemyActor) _activeperception)
        (if (not (Variables|Default|GetWasValidTarget))
          (AI|Components|Blackboard|SetValueasVector _returnvalue (Utilities|Name|MakeLiteralName "LOSAcquiredLocation") (Transformation|GetActorLocation (Pawn|GetControlledPawn)))
          (Variables|Default|SetWasValidTarget true))
        (elif (not (Utilities|Time|IsValidTimerHandle (Variables|Default|GetEnemyTimer)))
          (bind _returnvalue_2 (Utilities|Time|SetTimerbyEvent (delegate Custom|StartEnemyTimer) (Variables|Default|GetLineOfSightTimer)))
          (Variables|Default|SetEnemyTimer _returnvalue_2))))
    (:then_1
      (bind _distance (CallFunction|GetIdealSenseDistance)) ; Ramp up the current sense distance over time so we can flick torch on/off fast without alerting
      (Variables|Default|SetCurrentSenseDistance (select (> _distance (Variables|Default|GetCurrentSenseDistance)) (Math|Float|Lerp (Variables|Default|GetCurrentSenseDistance) _distance (* DeltaSeconds 1.7)) (Math|Float|Lerp (Variables|Default|GetCurrentSenseDistance) _distance (* DeltaSeconds 0.6)))))
    (:then_2
      (AI|Components|Blackboard|SetValueasBool (AI|GetBlackboard 0) (Utilities|Name|MakeLiteralName "LOSChaseBeyondRange") (> (Math|Vector|Distance(Vector) (Transformation|GetActorLocation (Pawn|GetControlledPawn)) (AI|Components|Blackboard|GetValueasVector (AI|GetBlackboard 0) (Utilities|Name|MakeLiteralName "LOSAcquiredLocation"))) 6e+02)))))

(event EventPossess
  (params (PossessedPawn :type Pawn%20Object%20Reference))
  (bind _returnvalue (AI|GetBlackboard 0))
  (AI|RunBehaviorTree "/Game/GBJam/Objects/Enemies/BP_EnemyBehaviourTree.BP_EnemyBehaviourTree")
  (bind _asbp_enemy (Utilities|Casting|CastToBP_Enemy PossessedPawn))
  (AI|Components|Blackboard|SetValueasVector _returnvalue (Utilities|Name|MakeLiteralName "BaseLocation") (Variables|/Game/GBJam/Objects/Enemies/BP_Enemy.BP_Enemy_C|GetBaseLocation _asbp_enemy))
  (AI|Components|Blackboard|SetValueasBool _returnvalue (Utilities|Name|MakeLiteralName "CanDamage") (Variables|/Game/GBJam/Objects/Enemies/BP_Enemy.BP_Enemy_C|GetCanDamage _asbp_enemy)))

(fn ConstructionScript)

(fn SetIsLightnear
  (params (Lightnear :type Boolean))
  (Variables|Default|SetNearLight Lightnear))

(fn IsValidTarget
  (params (Actor :type Actor%20Object%20Reference))
  (if (== Actor 0)
    (return false)
    (else
      (return (and (Actor|ActorHasTag Actor "Player") (< (Transformation|GetDistanceTo Actor (Pawn|GetControlledPawn)) (Variables|Default|GetCurrentSenseDistance)))))))

(fn NotifyFlashBombed
  (Utilities|Time|ClearandInvalidateTimerbyHandle (Variables|Default|GetFlashbombTimer))
  (AI|Components|Blackboard|SetValueasBool (AI|GetBlackboard 0) (Variables|Default|GetFlashbombedName) true)
  (bind _asbp_enemy (Utilities|Casting|CastToBP_Enemy (Pawn|GetControlledPawn)))
  (Default|SetIsFlashbombed _asbp_enemy true)
  (Utilities|Time|SetTimerbyEvent (EventDispatchers|CreateEvent :!event FlashbombComplete) (Variables|Default|GetFlashbombDuration)))

(fn FlashbombComplete
  (AI|Components|Blackboard|SetValueasBool (AI|GetBlackboard 0) (Variables|Default|GetFlashbombedName) false)
  (bind _asbp_enemy (Utilities|Casting|CastToBP_Enemy (Pawn|GetControlledPawn)))
  (Default|SetIsFlashbombed _asbp_enemy false))

(fn GetIdealSenseDistance
  (return (Math|Float|SelectFloat (Variables|Default|GetLightSenseDistance) (Variables|Default|GetSenseDistance) (Variables|Default|GetNearLight))))