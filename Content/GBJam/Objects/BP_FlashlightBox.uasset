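; BP_FlashlightBox is an interactable pickup box that refills the player's flashbombs up to MaxFlashbombs, despite its flashlight name.
; Its InteractBox overlaps register and unregister it as an interactable for the player character, with a pickup prompt.
; On interact, it spawns a BP_Flashbomb holding the missing count and immediately calls Interact on it, or shows a message when the player is full.
; The box is never consumed.
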(event OnComponentEndOverlap(InteractBox)
  (params (OverlappedComponent :type Primitive%20Component%20Object%20Reference) (OtherActor :type Actor%20Object%20Reference) (OtherComp :type Primitive%20Component%20Object%20Reference) (OtherBodyIndex :type Integer))
  (Utilities|Casting|CastToBP_PlayerCharacter OtherActor)
  (Class|GBGameplayStatics|RemoveInteractable self))

(event OnComponentBeginOverlap(InteractBox)
  (params (OverlappedComponent :type Primitive%20Component%20Object%20Reference) (OtherActor :type Actor%20Object%20Reference) (OtherComp :type Primitive%20Component%20Object%20Reference) (OtherBodyIndex :type Integer) (bFromSweep :type Boolean) (SweepResult :type Hit%20Result%20Structure%20%28by%20ref%29))
  (Utilities|Casting|CastToBP_PlayerCharacter OtherActor)
  (Class|GBGameplayStatics|AddInteractable self))

(event EventBeginPlay)

(event Collision|EventActorBeginOverlap
  (params (OtherActor :type Actor%20Object%20Reference)))

(event EventTick
  (params (DeltaSeconds :type Float%20%28single-precision%29)))

(event EventInteract
  (bind _asbp_player_character (Utilities|Casting|CastToBP_PlayerCharacter (Game|GetPlayerCharacter 0)))
  (bind _returnvalue (Class|GBJamCharacter|GetItemUsesLeft _asbp_player_character "/Game/GBJam/Objects/BP_Flashbomb.BP_Flashbomb_C"))
  (if (> (- (Variables|Default|GetMaxFlashbombs) _returnvalue) 0)
    (bind _returnvalue_2 (Game|SpawnActorfromClass "/Game/GBJam/Objects/BP_Flashbomb.BP_Flashbomb_C" (Math|Transform|MakeTransform "0, 0, 0") "Undefined" 0 0))
    (Variables|/Game/GBJam/Objects/BP_Flashbomb.BP_Flashbomb_C|SetFlashbombCount _returnvalue_2 (- (Variables|Default|GetMaxFlashbombs) _returnvalue))
    (Class|GBInteractable|Interact _returnvalue_2)
    (else
      (Class|GBGameplayStatics|ShowMessageBox "You can't carry any more flashbombs."))))

(fn ConstructionScript)

(fn GetPrompt
  (return "Z - Pickup"))