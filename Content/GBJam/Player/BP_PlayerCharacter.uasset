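; Player character Blueprint for the GBJam game that handles feedback for health changes and triggers game over on death.
; Its HealthComponent's damage and heal delegates look up rows in DT_Palettes, briefly flash that palette through the GBPaletteSubSystem and play a matching sound.
; On death it waits briefly so the damage flash can show, then calls GameOver on BP_GameMode.
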(event OnDeathDelegate(HealthComponent)
  (params (HealthComponent :type %20Object%20Reference) (DamageEvent :type Damage%20Event%20Structure%20%28by%20ref%29))
  (Utilities|FlowControl|Delay 0.2) ; Leave enough time for damage flash to occur
  (bind _asbp_game_mode (Utilities|Casting|CastToBP_GameMode (Game|GetGameMode)))
  (Default|GameOver _asbp_game_mode))

(event OnDamageDelegate(HealthComponent)
  (params (HealthComponent :type %20Object%20Reference) (DamageEvent :type Damage%20Event%20Structure%20%28by%20ref%29))
  (bind _returnvalue (Utilities|GetDataTableRow "/Game/GBJam/Palette/DT_Palettes.DT_Palettes" "Damage")
    (:then
      (Class|GBPaletteSubSystem|FlashPalette (Subsystems|GetGBPaletteSubSystem) _returnvalue 0.08)
      (Audio|PlaySound2D "/Game/GBJam/SFX/damage.damage" 1.0 1.0 0.0 0 0))))

(event OnHealDelegate(HealthComponent)
  (params (HealthComponent :type %20Object%20Reference) (DamageEvent :type Damage%20Event%20Structure%20%28by%20ref%29))
  (bind _returnvalue (Utilities|GetDataTableRow "/Game/GBJam/Palette/DT_Palettes.DT_Palettes" "Heal")
    (:then
      (Class|GBPaletteSubSystem|FlashPalette (Subsystems|GetGBPaletteSubSystem) _returnvalue 0.1)
      (Audio|PlaySound2D "/Game/GBJam/SFX/heal.heal" 1.0 1.0 0.0 0 0))))

(fn ConstructionScript)