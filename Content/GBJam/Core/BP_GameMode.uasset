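; Game mode for a GB Jam game that runs screen flow between title, in-game, game over and game complete.
; Each transition steps the palette to FadeOut via GBPaletteSubSystem, then switches HUD state and palette from DT_Palettes, toggling HUD focus to gate player control.
; Game over and completion reload the level, with GameInstance flags telling BeginPlay to show the end screen before returning to title.
; UpdateMusic only fetches the HUD.
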(event Custom|InGame
  ;[1 1 1] Fade out screen
  (bind _returnvalue (Utilities|GetDataTableRow "/Game/GBJam/Palette/DT_Palettes.DT_Palettes" "FadeOut")
    (:then
      (Class|GBPaletteSubSystem|TransitionPalette (Subsystems|GetGBPaletteSubSystem) _returnvalue 5 0.2)
      (Utilities|FlowControl|Delay 1.5)
      ;[1 1 1] Switch to ingame
      (bind _returnvalue_2 (Class|GBGameplayStatics|GetHUD))
      (Class|GBHUD|SetState _returnvalue_2 "InGame")
      ;[1 1 1] Fade screen back in
      (bind _returnvalue_3 (Utilities|GetDataTableRow "/Game/GBJam/Palette/DT_Palettes.DT_Palettes" "Default")
        (:then
          (Class|GBPaletteSubSystem|SetPalette (Subsystems|GetGBPaletteSubSystem) _returnvalue_3)
          ;[1 1 1] Release player control, which menu would have blocked
          (bind _returnvalue_4 (Class|GBGameplayStatics|GetHUD))
          (Class|GBHUD|ReleaseAllFocus _returnvalue_4)
          (CallFunction|UpdateMusic))))))

(event Custom|GameComplete
  ;[1 1 1] Prevent player control
  (bind _returnvalue (Class|GBGameplayStatics|GetHUD))
  (Class|GBHUD|TakeFocus _returnvalue)
  ;[1 1 1] Fade out screen
  (bind _returnvalue_2 (Utilities|GetDataTableRow "/Game/GBJam/Palette/DT_Palettes.DT_Palettes" "FadeOut")
    (:then
      (Class|GBPaletteSubSystem|TransitionPalette (Subsystems|GetGBPaletteSubSystem) _returnvalue_2 5 0.2)
      (Utilities|FlowControl|Delay 1.5)
      (bind _asbp_game_instance (Utilities|Casting|CastToBP_GameInstance (Game|GetGameInstance)))
      (Variables|/Game/GBJam/Core/BP_GameInstance.BP_GameInstance_C|SetLevelRestarting _asbp_game_instance true)
      (Variables|/Game/GBJam/Core/BP_GameInstance.BP_GameInstance_C|SetGameComplete _asbp_game_instance true)
      ;[1 1 1] Restart Level
      (bind _returnvalue_3 (Game|GetCurrentLevelName true))
      (Game|OpenLevel(byName) (Utilities|String|StringToName _returnvalue_3)))))

(event Custom|GameOver
  ;[1 1 1] Prevent player control
  (bind _returnvalue (Class|GBGameplayStatics|GetHUD))
  (Class|GBHUD|TakeFocus _returnvalue)
  ;[1 1 1] Fade out screen
  (bind _returnvalue_2 (Utilities|GetDataTableRow "/Game/GBJam/Palette/DT_Palettes.DT_Palettes" "FadeOut")
    (:then
      (Class|GBPaletteSubSystem|TransitionPalette (Subsystems|GetGBPaletteSubSystem) _returnvalue_2 5 0.2)
      (Utilities|FlowControl|Delay 1.5)
      (bind _asbp_game_instance (Utilities|Casting|CastToBP_GameInstance (Game|GetGameInstance)))
      (Variables|/Game/GBJam/Core/BP_GameInstance.BP_GameInstance_C|SetLevelRestarting _asbp_game_instance true)
      (Variables|/Game/GBJam/Core/BP_GameInstance.BP_GameInstance_C|SetGameComplete _asbp_game_instance false)
      ;[1 1 1] Restart Level
      (bind _returnvalue_3 (Game|GetCurrentLevelName true))
      (Game|OpenLevel(byName) (Utilities|String|StringToName _returnvalue_3)))))

(event Custom|Titlescreen
  ;[1 1 1] Prevent player control
  (bind _returnvalue (Class|GBGameplayStatics|GetHUD))
  (Class|GBHUD|TakeFocus _returnvalue)
  ;[1 1 1] Fade out screen
  (bind _returnvalue_2 (Utilities|GetDataTableRow "/Game/GBJam/Palette/DT_Palettes.DT_Palettes" "FadeOut")
    (:then
      (Class|GBPaletteSubSystem|TransitionPalette (Subsystems|GetGBPaletteSubSystem) _returnvalue_2 5 0.2)
      (Utilities|FlowControl|Delay 1.5)
      ;[1 1 1] Switch to titlescreen ui
      (bind _returnvalue_3 (Class|GBGameplayStatics|GetHUD))
      (Class|GBHUD|SetState _returnvalue_3 "TitleScreen")
      ;[1 1 1] Fade screen back in
      (bind _returnvalue_4 (Utilities|GetDataTableRow "/Game/GBJam/Palette/DT_Palettes.DT_Palettes" "TitleScreen")
        (:then
          (Class|GBPaletteSubSystem|SetPalette (Subsystems|GetGBPaletteSubSystem) _returnvalue_4)
          (CallFunction|UpdateMusic))))))

(event Custom|FinishLevelRestart
  (bind _asbp_game_instance (Utilities|Casting|CastToBP_GameInstance (Game|GetGameInstance)))
  ;[1 1 1] Switch to game over ui
  (bind _returnvalue (Class|GBGameplayStatics|GetHUD))
  (Class|GBHUD|SetState _returnvalue (select (Variables|/Game/GBJam/Core/BP_GameInstance.BP_GameInstance_C|GetGameComplete _asbp_game_instance) "GameComplete" "GameOver"))
  ;[1 1 1] Fade screen back in
  (bind _returnvalue_2 (Utilities|GetDataTableRow "/Game/GBJam/Palette/DT_Palettes.DT_Palettes" (select (Variables|/Game/GBJam/Core/BP_GameInstance.BP_GameInstance_C|GetGameComplete _asbp_game_instance) "GameComplete" "GameOver"))
    (:then
      (Class|GBPaletteSubSystem|SetPalette (Subsystems|GetGBPaletteSubSystem) _returnvalue_2)
      (Utilities|FlowControl|Delay 3.0)
      ;[1 1 1] Release player control
      (bind _returnvalue_3 (Class|GBGameplayStatics|GetHUD))
      (Class|GBHUD|TakeFocus _returnvalue_3)
      (bind _asbp_game_instance_2 (Utilities|Casting|CastToBP_GameInstance (Game|GetGameInstance)))
      (Variables|/Game/GBJam/Core/BP_GameInstance.BP_GameInstance_C|SetLevelRestarting _asbp_game_instance_2 false)
      (CallFunction|Titlescreen))))

(event Custom|UpdateMusic
  (Class|GBGameplayStatics|GetHUD))

(event EventBeginPlay
  (bind _asbp_game_instance (Utilities|Casting|CastToBP_GameInstance (Game|GetGameInstance)))
  (if (Variables|/Game/GBJam/Core/BP_GameInstance.BP_GameInstance_C|GetLevelRestarting _asbp_game_instance)
    (CallFunction|FinishLevelRestart)
    (else
      ;[1 1 1] Apply default palette
      (bind _returnvalue (Utilities|GetDataTableRow "/Game/GBJam/Palette/DT_Palettes.DT_Palettes" "Default")
        (:then
          (Class|GBPaletteSubSystem|SetPalette (Subsystems|GetGBPaletteSubSystem) _returnvalue)
          (CallFunction|UpdateMusic))))))

(event EventTick
  (params (DeltaSeconds :type Float%20%28single-precision%29)))

(fn ConstructionScript)

(fn UpdateMaterialPalettes)