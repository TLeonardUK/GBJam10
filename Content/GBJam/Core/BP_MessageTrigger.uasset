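; BP_MessageTrigger is a trigger volume that shows a list of message boxes to the player.
; When the player character enters its box, it either fires immediately or, if interaction is required, registers itself as an interactable with a prompt until the player leaves.
; An optional once-only flag stops it from showing its messages again after it has triggered.
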(event OnComponentBeginOverlap(Box)
  (params (OverlappedComponent :type Primitive%20Component%20Object%20Reference) (OtherActor :type Actor%20Object%20Reference) (OtherComp :type Primitive%20Component%20Object%20Reference) (OtherBodyIndex :type Integer) (bFromSweep :type Boolean) (SweepResult :type Hit%20Result%20Structure%20%28by%20ref%29))
  (Utilities|Casting|CastToBP_PlayerCharacter OtherActor)
  (if (Variables|Default|GetNeedsInteract)
    (if (CallFunction|IsTriggerable)
      (Class|GBGameplayStatics|AddInteractable self))
    (else
      (CallFunction|Trigger))))

(event OnComponentEndOverlap(Box)
  (params (OverlappedComponent :type Primitive%20Component%20Object%20Reference) (OtherActor :type Actor%20Object%20Reference) (OtherComp :type Primitive%20Component%20Object%20Reference) (OtherBodyIndex :type Integer))
  (Utilities|Casting|CastToBP_PlayerCharacter OtherActor)
  (Class|GBGameplayStatics|RemoveInteractable self))

(event Custom|Trigger
  (if (CallFunction|IsTriggerable)
    (for _array_element (Variables|Default|GetMessages)
      (Class|GBGameplayStatics|ShowMessageBox _array_element))
    (Variables|Default|SetHasTriggered true)))

(event EventBeginPlay)

(event Collision|EventActorBeginOverlap
  (params (OtherActor :type Actor%20Object%20Reference)))

(event EventTick
  (params (DeltaSeconds :type Float%20%28single-precision%29)))

(event EventInteract
  (CallFunction|Trigger))

(fn ConstructionScript)

(fn IsTriggerable
  (return (or (not (Variables|Default|GetOnceOnly)) (not (Variables|Default|GetHasTriggered)))))

(fn GetPrompt
  (return (Variables|Default|GetInteractPrompt)))