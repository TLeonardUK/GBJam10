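; BP_VelocitySound plays random sounds from its owner while that owner moves faster than a minimum velocity.
; A looping timer started on BeginPlay checks the velocity of the owner's MovementComponent at a set interval.
; When the speed exceeds the threshold, it picks a random entry from the Audio array and plays it at the owner's location.
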(event Custom|Sound
  (bind _returnvalue (Components|GetOwner))
  (bind _returnvalue_2 (Actor|GetComponentbyClass _returnvalue "/Script/Engine.MovementComponent"))
  (Utilities|IsValid _returnvalue_2
    (:Is%20Valid
      (if (> (Math|Vector|VectorLength (Variables|/Script/Engine.MovementComponent|GetVelocity _returnvalue_2)) (Variables|Default|GetMinimumVelocity))
        (Audio|PlaySoundatLocation (.OutItem (Utilities|Array|Random (Variables|Default|GetAudio))) (Transformation|GetActorLocation _returnvalue) "0, 0, 0" 1.0 1.0 0.0 0 0 0 0)))))

(event EventBeginPlay
  (Utilities|Time|SetTimerbyEvent (delegate Custom|Sound) (Variables|Default|GetInterval) true))

(event EventTick
  (params (DeltaSeconds :type Float%20%28single-precision%29)))